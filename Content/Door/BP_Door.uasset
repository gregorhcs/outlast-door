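; BP_Door is an interactable door that swings with left/right axis input while held, or auto-opens after a brief interaction.
; It drives a RotatingMovement component's yaw rate, using the RateDecay timeline to taper the speed after each input.
; Tick stops rotation at the open and closed angle limits.
; Interaction events inherited from its parent show and hide a WB_DoorInteraction prompt and time the press.
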(event `self.ReceiveBeginPlay`
  ;[0 0 0] Begin Play
  (`|ExecutionSequence`
    (:`then_0`
      ;;[0.2292 0.2292 0.2292] Create Open/Close Door Widget
      (bind _returnvalue (`|CreateWidget` "/Game/Door/WB_DoorInteraction.WB_DoorInteraction_C"))
      (bind _output_get (set `self.WB_InteractionUI` _returnvalue))
      (`UserWidget.AddToViewport` _output_get 0)
      (`Widget.SetVisibility` _output_get "Hidden"))
    (:`then_1`
      ;;[0.2292 0.2292 0.2292] Bind Show Hide UI
      (add `self.OnCanInteractNow` (delegate `ShowInteractionUI`)))
    (:`then_2`
      (add `self.OnCanInteractNoLonger` (delegate `HideInteractionUI`)))))

(event `ShowInteractionUI`
  ;[0 0 0] Begin Play
  ;;[0.2292 0.2292 0.2292] Bind Show Hide UI
  (`Widget.SetVisibility` (`self.WB_InteractionUI`) "Visible"))

(event `HideInteractionUI`
  ;[0 0 0] Begin Play
  ;;[0.2292 0.2292 0.2292] Bind Show Hide UI
  (`Widget.SetVisibility` (`self.WB_InteractionUI`) "Hidden"))

(event `/Game/Door/BI_InteractionProvider.InteractionStart`
  (params (Interactor :type "Actor Object Reference"))
  ;[0 0 0] Interaction Start/Stop
  (`parent.InteractionStart` Interactor)
  (set `self.TimeInteractionStart` (`GameplayStatics.GetTimeSeconds`)))

(event `/Game/Door/BI_InteractionProvider.InteractionStop`
  (params (Interactor :type "Actor Object Reference"))
  ;[0 0 0] Interaction Start/Stop
  (`parent.InteractionStop` Interactor)
  (`self.SetRotationRateZ` 0.0)
  (if (and (< (- (`GameplayStatics.GetTimeSeconds`) (`self.TimeInteractionStart`)) (`self.AutoOpenTimeThreshold`)) (not (`self.DoorTooFarOpen?`)))
    (`self.SetRotationRateZ` (`self.AutopOpenSpeed`))))

(event `/Game/Door/BI_AxisTickOvserver.TickAxisUp`
  (params (AxisUpValue :type "Float (double-precision)"))
  ;[0 0 0] Axis Tick
)

(event `/Game/Door/BI_AxisTickOvserver.TickAxisRight`
  (params (AxisRightValue :type "Float (double-precision)"))
  ;[0 0 0] Axis Tick
  (if (`self.IsInteracting?`)
    (if (> (`KismetMathLibrary.Abs` AxisRightValue) (`self.MinLeftRightMovement`))
      (if (> AxisRightValue 0.0)
        (if (not (`self.DoorTooFarClosed?`))
          (set `self.DoorSpeed` (* -1.0 (`self.DefaultDoorSpeed`)))
          (`self.SetRotationRateZ` (`self.DoorSpeed`))
          (bind (_direction _alpha) (`Timeline|RateDecay` :!via `PlayFromStart` :!label _label)
            (:`Update`
              (`self.SetRotationRateZ` (* _alpha (`self.DoorSpeed`))))))
        (elif (not (`self.DoorTooFarOpen?`))
          (set `self.DoorSpeed` (`self.DefaultDoorSpeed`))
          (`self.SetRotationRateZ` (`self.DoorSpeed`))
          (goto _label :!via `PlayFromStart`))))))

(event `self.ReceiveTick`
  (params (DeltaSeconds :type "Float (single-precision)"))
  ;[0 0 0] Axis Tick
  (if (or (and (`self.DoorTooFarOpen?`) (> (.yaw (`RotatingMovementComponent.RotationRate` (`self.RotatingMovement`))) 0.0)) (and (`self.DoorTooFarClosed?`) (< (.yaw (`RotatingMovementComponent.RotationRate` (`self.RotatingMovement`))) 0.0)))
    (`TimelineComponent.Stop` (`self.RateDecay`))
    (`self.SetRotationRateZ` 0.0)))

(fn `UserConstructionScript`)